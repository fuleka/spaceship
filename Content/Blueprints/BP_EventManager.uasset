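; BP_EventManager is an event hub that creates the main HUD and turns game messages into state variables.
; On BeginPlay it binds a handler to the message-send event and adds BP_MainHUD to the viewport.
; Item pickup messages set toast text and raise an update flag, while stage-start messages store the stage count.
; Tick caches the player pawn's location every frame.
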(event `self.ReceiveBeginPlay`
  (add `self.MesageSend` (delegate `MesageSend_Event`))
  (bind _returnvalue (`|CreateWidget` "/Game/Blueprints/Widget/BP_MainHUD.BP_MainHUD_C" (`GameplayStatics.GetPlayerController` 0)))
  (`UserWidget.AddToViewport` _returnvalue 0))

(event `MesageSend_Event` :!signature `self.MesageSend`
  (params (MesageType :type "/Game/Blueprints/Table/En_MesageType Enum" :default "NewEnumerator0") (Value :type Integer))
  (switch `/Game/Blueprints/Table/En_MesageType` MesageType
    (:`NewEnumerator2`
      (set `self.ToastMent` (`|FormatText` "Player Get Item ({value})" Value))
      (set `self.PlzToastUpdate` true))
    (:`NewEnumerator4`
      (set `self.StageCount` Value))))

(event `self.ReceiveTick`
  (params (DeltaSeconds :type "Float (single-precision)"))
  (bind _returnvalue_location (`KismetMathLibrary.BreakTransform` (`self.GetTransform` (`GameplayStatics.GetPlayerPawn` 0))))
  (set `self.PlayerLocation` _returnvalue_location))

(fn `UserConstructionScript`)