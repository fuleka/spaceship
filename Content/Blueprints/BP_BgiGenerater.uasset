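; BP_BgiGenerater is an actor that builds a tiled arrangement of Paper2D sprites, apparently a test background image generator.
; BeginPlay adds the sprite components at runtime, places them using X/Z offsets from SpriteSetVec at a fixed Y depth, and assigns a test sprite.
; The construction script tints the SprtieTmp array, which this file only fills at BeginPlay.
; Tick caches the player pawn's location, which is not used here.
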(event `self.ReceiveBeginPlay`
  (`parent.ReceiveBeginPlay`)
  (for _ (range 9)
    (bind _returnvalue (`AddComponent|NODE_AddPaperSpriteComponent-1` :`self` self))
    (`KismetArrayLibrary.Array_Add` (`self.SprtieTmp`) _returnvalue))
  (for (_array_element _array_index) (`self.SprtieTmp`)
    (bind _value (`BlueprintMapLibrary.Map_Find` (`self.SpriteSetVec`) _array_index))
    (`SceneComponent.K2_SetRelativeLocationAndRotation` :`self` _array_element :`NewLocation` (`KismetMathLibrary.MakeVector` (.x _value) -200.0 (.z _value)))
    (`PaperSpriteComponent.SetSprite` _array_element "/Game/BackgrondImg/testBgi_Sprite.testBgi_Sprite")))

(event `self.ReceiveTick`
  (params (DeltaSeconds :type "Float (single-precision)"))
  (`parent.ReceiveTick` DeltaSeconds)
  (set `self.PlayerLocation` (`self.K2_GetActorLocation` (`GameplayStatics.GetPlayerPawn` 0))))

(fn `UserConstructionScript`
  (locals (testcolor :type "LinearColor Structure" :default (struct)))
  (`parent.UserConstructionScript`)
  (for _array_element (`self.SprtieTmp`)
    (`PaperSpriteComponent.SetSpriteColor` _array_element (`local.testcolor`))))