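; Gun Blueprint that fires repeatedly from its owner, using a Delay on Tick as the attack interval.
; Projectile mode spawns BP_Projectile at a named socket, aimed at the nearest target-class actor on the XZ plane or by Front, Back or Side setting.
; Each projectile receives damage, speed and a point-or-radius flag.
; Trace mode line-traces Pawns along the owner's up vector and only spawns an explosion effect on hit.
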(event `self.ReceiveBeginPlay`)

(event `self.ReceiveTick`
  (params (DeltaSeconds :type "Float (single-precision)"))
  (bind _gunowner (`self.GunOwner`))
  (bind _gunowner_2 (`self.GunOwner`))
  (bind _gunowner_3 (`self.GunOwner`))
  (bind _returnvalue (`Actor.K2_GetActorLocation` _gunowner))
  (bind _returnvalue_2 (`Actor.K2_GetActorLocation` (`self.GunOwner`)))
  (bind _returnvalue_location (`KismetMathLibrary.BreakTransform` (`SceneComponent.GetSocketTransform` (`Actor.RootComponent` (`self.GunOwner`)) (`self.SoketName`) "RTS_World")))
  (bind _returnvalue_3 (`SceneComponent.K2_GetComponentRotation` (`Actor.RootComponent` (`self.GunOwner`))))
  (bind _returnvalue_location_2 (`KismetMathLibrary.BreakTransform` (`SceneComponent.GetSocketTransform` (`Actor.RootComponent` (`self.GunOwner`)) (`self.SoketName`) "RTS_World")))
  (`KismetSystemLibrary.Delay` (`self.AttackDelay`))
  (switch `/Game/Blueprints/Table/En_WeaponType` (`self.WeaponType`)
    (:`NewEnumerator0`
      (switch `/Game/Blueprints/Table/En_TargetType` (`self.TargetType`)
        (:`NewEnumerator0`
          (bind (_targetactorref _isnotvaild) (`self.GetFireTarget` (`self.TargetClass`) _returnvalue_2))
          (if (not _isnotvaild)
            (`self.SpawnProjectile` "/Game/Blueprints/Unit/BP_Projectile.BP_Projectile_C" _returnvalue_2 (`Actor.K2_GetActorLocation` _targetactorref) (0.3 0.3 0.3))))
        (:`NewEnumerator1`
          (set `self.ShootDirection` _returnvalue_3 :!label _label)
          (bind `_as폰` (cast `Pawn` _gunowner_2 :!label _label_2))
          (`self.SpawnedProjectileSetting` "/Game/Blueprints/Unit/BP_Projectile.BP_Projectile_C" `_as폰` _gunowner_2 (`KismetMathLibrary.MakeTransform` _returnvalue_location_2 (`self.ShootDirection`) (0.3 0.3 0.3))))
        (:`NewEnumerator4`
          (set `self.ShootDirection` (* _returnvalue_3 -1.0))
          (goto _label_2))
        (:`NewEnumerator2`
          (switch `name` (`self.SoketName`)
            (:`Left`
              (set `self.ShootDirection` (`KismetMathLibrary.NormalizedDeltaRotator` (`SceneComponent.K2_GetComponentRotation` (`Actor.RootComponent` (`self.GunOwner`))) (struct :`Pitch` -90.0))))
            (:`Right`
              (set `self.ShootDirection` (`KismetMathLibrary.NormalizedDeltaRotator` (`SceneComponent.K2_GetComponentRotation` (`Actor.RootComponent` (`self.GunOwner`))) (struct :`Pitch` 90.0))))
            (:`Front`
              (goto _label)))
          (bind `_as폰_2` (cast `Pawn` _gunowner_3))
          (`self.SpawnedProjectileSetting` "/Game/Blueprints/Unit/BP_Projectile.BP_Projectile_C" `_as폰_2` _gunowner_3 (`KismetMathLibrary.MakeTransform` _returnvalue_location (`self.ShootDirection`) (0.3 0.3 0.3))))))
    (:`NewEnumerator1`
      (bind _outhit (`KismetSystemLibrary.LineTraceSingleForObjects` _returnvalue (+ _returnvalue (* (`Actor.GetActorUpVector` _gunowner) (1000.0 1000.0 1000.0))) (`|MakeArray` "ObjectTypeQuery3" :!type "EObjectTypeQuery Enum") false (`|MakeArray` (`self.GunOwner`)) "ForOneFrame"))
      (bind (_bblockinghit _binitialoverlap _time _distance _location) (`GameplayStatics.BreakHitResult` _outhit))
      (if _bblockinghit
        (`GameplayStatics.SpawnEmitterAtLocation` "/Game/StarterContent/Particles/P_Explosion.P_Explosion" _location)))))

(fn `GetFireTarget`
  (params (TargetActorClass :type "Actor Class Reference") (OriginLoc :type "Vector Structure"))
  (returns (TargetActorRef :type "Actor Object Reference") (IsNotVaild :type Boolean))
  (locals (TargetList :type "Array of Actor Object Reference") (IsNotValid :type Boolean :default true))
  (bind _outactors (`GameplayStatics.GetAllActorsOfClass` TargetActorClass))
  (bind _output_get (set `local.TargetList` _outactors))
  (if (`KismetArrayLibrary.Array_IsNotEmpty` _output_get)
    (bind (_distance _returnvalue) (`GameplayStatics.FindNearestActor` OriginLoc _output_get))
    (`/Engine/EditorBlueprintResources/StandardMacros.IsValid` _returnvalue
      (:`Is Valid`
        (bind _output_get_2 (set `local.IsNotValid` false))
        (return _returnvalue _output_get_2))
      (:`Is Not Valid`
        _)))
  (`KismetSystemLibrary.PrintString` "Find Nearest Actor is Not Valid Actor call")
  (bind _output_get_3 (set `local.IsNotValid` true))
  (return _returnvalue _output_get_3))

(fn `SetAutoTargetDirection`
  (params (Origin :type "Vector Structure") (Target :type "Vector Structure"))
  (returns (ShootDirection :type "Rotator Structure"))
  (bind (_returnvalue_x _returnvalue_y _returnvalue_z) (`KismetMathLibrary.BreakVector` (- (`KismetMathLibrary.MakeVector` (.x Origin) 0.0 (.z Origin)) (`KismetMathLibrary.MakeVector` (.x Target) 0.0 (.z Target)))))
  (bind _output_get (set `self.ShootDirection` (`KismetMathLibrary.MakeRotator` 0.0 (+ (`KismetMathLibrary.DegAtan2` _returnvalue_z _returnvalue_x) 90.0 0.0))))
  (return _output_get))

(fn `SpawnedProjectileSetting`
  (params (Class :type "Actor Class Reference") (Instigator :type "Pawn Object Reference") (Owner :type "Actor Object Reference") (SpawnTransform :type "Transform Structure"))
  (bind _damagevalue (`self.DamageValue`))
  (bind _projectilespeed (`self.ProjectileSpeed`))
  (bind _returnvalue (`|SpawnActorFromClass` Class SpawnTransform "AdjustIfPossibleButAlwaysSpawn" "OverrideRootScale" Owner Instigator))
  (`/Engine/EditorBlueprintResources/StandardMacros.IsValid` _returnvalue
    (:`Is Valid`
      (switch `/Game/Blueprints/Table/En_DamageType` (`self.DamageType`)
        (:`NewEnumerator0`
          (message `/Game/Blueprints/BP_MainInterface.SetProjectileInfo` _returnvalue _damagevalue _projectilespeed false))
        (:`NewEnumerator1`
          (message `/Game/Blueprints/BP_MainInterface.SetProjectileInfo` _returnvalue _damagevalue _projectilespeed true))))))

(fn `SpawnProjectile`
  (params (ProjectileClass :type "Actor Class Reference") (Origin :type "Vector Structure") (TargetLoc :type "Vector Structure") (Scale :type "Vector Structure"))
  (bind _gunowner (`self.GunOwner`))
  (bind _shootdirection (`self.SetAutoTargetDirection` Origin TargetLoc))
  (bind `_as폰` (cast `Pawn` _gunowner))
  (`self.SpawnedProjectileSetting` ProjectileClass `_as폰` _gunowner (`KismetMathLibrary.MakeTransform` (.location (`SceneComponent.GetSocketTransform` (`Actor.RootComponent` (`self.GunOwner`)) (`self.SoketName`) "RTS_World")) _shootdirection Scale))
  (return))