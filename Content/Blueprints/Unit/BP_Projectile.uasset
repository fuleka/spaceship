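; Projectile actor that damages what it overlaps and spawns an explosion emitter when destroyed.
; BeginPlay caches the instigator's controller and makes projectile and instigator ignore each other when moving.
; On overlap, CanDamagedRadius adds a pawn sphere query; otherwise actors sharing the instigator controller are skipped.
; It applies DamageValue to the DamagedActor list, then DestroyReady destroys it or sets a short timer, depending on ReadyToDamageSet.
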(event `/Game/Blueprints/BP_MainInterface.SetProjectileInfo`
  (params (DamageValue :type "Float (double-precision)") (ProjectileSpeed :type "Float (double-precision)") (CanDamageRadius :type Boolean))
  ;[1 1 1] 코멘트
  (set `self.DamageValue` DamageValue)
  (set `self.ReadyToDamageSet` false))

(event `self.ReceiveBeginPlay`
  (set `self.RefInstigatorController` (`Pawn.GetController` (`self.Instigator`)))
  (`PrimitiveComponent.IgnoreActorWhenMoving` (`self.StaticMesh`) (`self.Instigator`) true)
  (`PrimitiveComponent.IgnoreActorWhenMoving` (`self.GetComponentByClass` (`self.Instigator`) "/Script/Engine.StaticMeshComponent") self true))

(event `self.ReceiveDestroyed`
  (`GameplayStatics.SpawnEmitterAtLocation` "/Game/StarterContent/Particles/P_Explosion.P_Explosion" (`self.K2_GetActorLocation`) (struct) (0.3 0.3 0.3)))

(event `self.ReceiveActorBeginOverlap`
  (params (OtherActor :type "Actor Object Reference"))
  (if (`self.CanDamagedRadius`)
    (bind _outactors (`KismetSystemLibrary.SphereOverlapActors` (0.0 0.0 0.0) 300.0 (`|MakeArray` (enumliteral `EObjectTypeQuery` "ObjectTypeQuery3"))))
    (`KismetArrayLibrary.Array_Append` _outactors (`self.DamagedActor`))
    (`KismetArrayLibrary.Array_AddUnique` (`self.DamagedActor`) OtherActor :!label _label)
    (for _array_element (`self.DamagedActor`)
      (`GameplayStatics.ApplyDamage` _array_element (`self.DamageValue`) (`self.RefInstigatorController`) self "/Game/Blueprints/BP_DamageType.BP_DamageType_C"))
    (`self.DestroyReady`)
    (elif (not (== (`self.GetInstigatorController` OtherActor) (`self.GetInstigatorController` self)))
      (goto _label))))

(fn `DestroyReady`
  (if (`self.ReadyToDamageSet`)
    (`KismetSystemLibrary.K2_SetTimer` null "DestroyReady" 0.25)
    (set `self.ReadyToDamageSet` true)
    (else
      (`self.K2_DestroyActor`))))

(fn `GetDamage`
  (params (DamageValue :type Integer))
  (return))

(fn `UserConstructionScript`)