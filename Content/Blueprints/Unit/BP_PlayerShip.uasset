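; Player-controlled ship that flies along its mesh's up vector, pitches on the vertical axis, and targets NPC ships with its guns.
; The Breaking action suppresses thrust input while held.
; Booster doubles acceleration and max speed until released, but never clears its Boosting flag, so it cannot re-trigger.
; Overlapping field items are collected through an interface check, and GoDestroy is left empty.
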(event `self.ReceiveBeginPlay`
  (`parent.ReceiveBeginPlay`)
  (`self.EnableInput` (`GameplayStatics.GetPlayerController` 0))
  (for _array_element (`self.GunList`)
    (set `/Game/Blueprints/Unit/BP_Gun.TargetClass` "/Game/Blueprints/Unit/BP_NpcShip.BP_NpcShip_C" _array_element)))

(event `InputAxis|MoveX`
  (params (AxisValue :type "Float (single-precision)"))
  (if (not (`self.IsBreaking`))
    (`self.AddMovementInput` (`SceneComponent.GetUpVector` (`self.Ship_StaticMesh`)) AxisValue)))

(event `InputAxis|MoveY`
  (params (AxisValue :type "Float (single-precision)"))
  (`SceneComponent.K2_AddWorldRotation` (`self.Ship_StaticMesh`) (`KismetMathLibrary.MakeRotator` 0.0 (* AxisValue -1.0)) false false))

(event `InputAction|Booster`
  (params (Key :type "Key Structure"))
  (bind _ship_floatingpawnmovement (`self.Ship_FloatingPawnMovement`))
  (bind _boosting (`self.Boosting`))
  (bind _ship_floatingpawnmovement_2 (`self.Ship_FloatingPawnMovement`))
  (:`Pressed`
    (if (not _boosting)
      (set `self.Boosting` true)
      (bind _output_get (set `self.AccTmp` (`FloatingPawnMovement.Acceleration` _ship_floatingpawnmovement)))
      (set `FloatingPawnMovement.Acceleration` (* _output_get 2.0) _ship_floatingpawnmovement)
      (bind _output_get_2 (set `self.MaxSpeedTmp` (`FloatingPawnMovement.MaxSpeed` _ship_floatingpawnmovement)))
      (set `FloatingPawnMovement.MaxSpeed` (* _output_get_2 2.0) _ship_floatingpawnmovement)))
  (:`Released`
    (if _boosting
      (set `FloatingPawnMovement.Acceleration` (`self.AccTmp`) _ship_floatingpawnmovement_2)
      (set `FloatingPawnMovement.MaxSpeed` (`self.MaxSpeedTmp`) _ship_floatingpawnmovement_2))))

(event `InputAction|Breaking`
  (params (Key :type "Key Structure"))
  (:`Pressed`
    (set `self.IsBreaking` true))
  (:`Released`
    (set `self.IsBreaking` false)))

(event `self.ReceiveActorBeginOverlap`
  (params (OtherActor :type "Actor Object Reference"))
  (`parent.ReceiveActorBeginOverlap` OtherActor)
  (if (`KismetSystemLibrary.DoesImplementInterface` OtherActor "/Game/Blueprints/BP_GetFieldItem.BP_GetFieldItem_C")
    (bind _asbp_field_item (cast `/Game/Blueprints/Unit/BP_FieldItem` OtherActor))
    (`/Game/Blueprints/BP_GetFieldItem.PlayerGet` _asbp_field_item)))

(event `self.ReceiveTick`
  (params (DeltaSeconds :type "Float (single-precision)"))
  (`parent.ReceiveTick` DeltaSeconds)
  (`|ExecutionSequence`))

(event `/Game/Blueprints/BP_MainInterface.GoDestroy`)

(fn `UserConstructionScript`
  (`parent.UserConstructionScript`))