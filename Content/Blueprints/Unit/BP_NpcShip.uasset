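; NPC enemy ship that follows the player, aims its guns at BP_PlayerShip and leaves a smoke effect when destroyed.
; Each Tick feeds player distance into PlayerChase, which pitches the ship toward the player through an atan2 angle.
; Beyond DetectRadius it moves along its up vector, forward vector or their sum by distance band; otherwise it backs away.
; Movement is a swept MoveUpdatedComponent step, not scaled by delta time.
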(event `self.ReceiveBeginPlay`
  (`parent.ReceiveBeginPlay`)
  (for _array_element (`self.GunList`)
    (set `/Game/Blueprints/Unit/BP_Gun.TargetClass` "/Game/Blueprints/Unit/BP_PlayerShip.BP_PlayerShip_C" _array_element)
    (set `self.Instigator` self)))

(event `self.ReceiveDestroyed`
  (`GameplayStatics.SpawnEmitterAtLocation` "/Game/StarterContent/Particles/P_Smoke.P_Smoke" (`self.K2_GetActorLocation`) (struct) (0.5 0.5 0.5)))

(event `self.ReceiveTick`
  (params (DeltaSeconds :type "Float (single-precision)"))
  (`parent.ReceiveTick` DeltaSeconds)
  (`|ExecutionSequence`
    (:`then_0`
      (set `self.DistanceByPlayer` (`KismetMathLibrary.Vector_Distance` (`self.K2_GetActorLocation` (`GameplayStatics.GetPlayerPawn` 0)) (`self.K2_GetActorLocation`)))
      (`self.PlayerChase` (> (`self.DistanceByPlayer`) (`self.DetectRadius`))))))

(event `/Game/Blueprints/BP_MainInterface.GoDestroy`
  (`self.K2_DestroyActor`))

(fn `PlayerChase`
  (params (FirstDistanceCheck :type Boolean))
  (locals (AddRotationValue :type Boolean) (HeadingVec :type "Vector Structure"))
  (bind _distancebyplayer (`self.DistanceByPlayer`))
  (if FirstDistanceCheck
    (set `self.Heading` 1.0)
    (if (>= _distancebyplayer 500.0)
      (set `local.HeadingVec` (`self.GetActorUpVector`))
      (elif (`KismetMathLibrary.InRange_FloatFloat` _distancebyplayer 400.0 500.0)
        (set `local.HeadingVec` (+ (`self.GetActorUpVector`) (`self.GetActorForwardVector`)))
        (else
          (set `local.HeadingVec` (`self.GetActorForwardVector`)))))
    (else
      (set `self.Heading` -1.0)
      (set `local.HeadingVec` (`self.GetActorUpVector`))))
  (`MovementComponent.K2_MoveUpdatedComponent` (`self.Ship_FloatingPawnMovement`) (* (`local.HeadingVec`) (`self.Speed`) (`self.Heading`)) (`KismetMathLibrary.MakeRotator` 0.0 (`/Game/Blueprints/Actor_Mac.Angle_Atan2` (`self.K2_GetActorLocation`) (`self.K2_GetActorLocation` (`GameplayStatics.GetPlayerPawn` 0)))) true false))

(fn `UserConstructionScript`
  (`parent.UserConstructionScript`))