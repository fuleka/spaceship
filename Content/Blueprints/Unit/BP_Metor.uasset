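; BP_Metor is a meteor projectile that reports hits on the player and destroys itself on impact.
; On BeginPlay it sets its ProjectileMovement velocity along local Z from Speed and caches the GameState as BP_EventManager.
; A mesh hit on the player pawn sends a typed message with a value through that manager, and any hit destroys the meteor, including one with another meteor.
; A separate GoDestroy event also destroys it.
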(event `self.ReceiveTick`
  (params (DeltaSeconds :type "Float (single-precision)")))

(event `self.ReceiveBeginPlay`
  (`self.SetSpeed`)
  (bind _asbp_event_manager (cast `/Game/Blueprints/BP_EventManager` (`GameplayStatics.GetGameState`)))
  (set `self.Ref_Manager` _asbp_event_manager))

(event `self.ReceiveActorBeginOverlap`
  (params (OtherActor :type "Actor Object Reference")))

(event `/Game/Blueprints/BP_MainInterface.GoDestroy`
  (`self.K2_DestroyActor`))

(event `self.StaticMesh.OnComponentHit`
  (params (HitComponent :type "PrimitiveComponent Object Reference") (OtherActor :type "Actor Object Reference") (OtherComp :type "PrimitiveComponent Object Reference") (NormalImpulse :type "Vector Structure") (Hit :type "HitResult Structure (by ref)"))
  (if (== (`GameplayStatics.GetObjectClass` OtherActor) (`GameplayStatics.GetObjectClass` self))
    _
    (elif (== OtherActor (`GameplayStatics.GetPlayerPawn` 0))
      (`/Game/Blueprints/BP_EventManager.MesageSend` (`self.Ref_Manager`) "NewEnumerator1" 1)))
  (`self.K2_DestroyActor`))

(fn `SetSpeed`
  (`ProjectileMovementComponent.SetVelocityInLocalSpace` (`self.ProjectileMovement`) (`KismetMathLibrary.MakeVector` 0.0 0.0 (`self.Speed`))))

(fn `UserConstructionScript`)