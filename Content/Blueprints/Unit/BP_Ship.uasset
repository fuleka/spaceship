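; Ship unit Blueprint that handles health, data-driven setup and weapons.
; SetShipInfo loads mesh and HP from DT_ShipInfo, feeding the default item to player-state inventory, while AddWeapon creates configured BPGun components from DT_WeaponInfo sockets.
; Incoming damage passes a BP_DamageType target filter; lethal hits only destroy the ship when player-instigated, notifying BP_EventManager on the GameState.
; Helpers find nearest targets and spawn pitch-aimed projectiles from the Fire socket.
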(event `self.ReceiveAnyDamage`
  (params (Damage :type "Float (single-precision)") (DamageType :type "DamageType Object Reference") (InstigatedBy :type "Controller Object Reference") (DamageCauser :type "Actor Object Reference"))
  (bind (_returnvalue_x _returnvalue_y _returnvalue_z) (`KismetMathLibrary.BreakVector` (`self.K2_GetActorLocation` self)))
  (bind _returnvalue (- (`self.CurrentHp`) Damage))
  (bind _asbp_damage_type (cast `/Game/Blueprints/BP_DamageType` DamageType))
  (bind _sameclass (`/Game/Blueprints/BP_DamageType.TargetFilter` _asbp_damage_type InstigatedBy (`self.GetController` self)))
  (if _sameclass
    _
    (elif (<= _returnvalue 0.0)
      (`/Engine/EditorBlueprintResources/StandardMacros.IsValid` InstigatedBy
        (:`Is Valid`
          (if (`Controller.IsPlayerController` InstigatedBy)
            (`/Game/Blueprints/BP_EventManager.MesageSend_Event` (`self.RefEventManager`) "NewEnumerator3" 1 (`KismetMathLibrary.MakeVector2D` _returnvalue_x _returnvalue_z))
            (`/Game/Blueprints/BP_MainInterface.GoDestroy` self))))
      (else
        (set `self.CurrentHp` _returnvalue)))))

(event `self.ReceiveBeginPlay`
  (`|ExecutionSequence`
    (:`then_1`
      (bind _asbp_event_manager (cast `/Game/Blueprints/BP_EventManager` (`GameplayStatics.GetGameState`)))
      (set `self.RefEventManager` _asbp_event_manager))))

(event `self.ReceiveTick`
  (params (DeltaSeconds :type "Float (single-precision)")))

(event `WeaponGet`)

(event `WeaponDelet`
  (for _array_element (`self.GunList`)
    _))

(event `/Game/Blueprints/BP_MainInterface.SendShipInfo`
  (params (ShipName :type Name))
  (bind _itemname (`self.SetShipInfo` ShipName))
  (bind _asbp_player_state (cast `/Game/Blueprints/BP_PlayerState` (`GameplayStatics.GetPlayerState` 0)))
  (`/Game/Blueprints/BP_PlayerState.RefreshInventory` _asbp_player_state _itemname)
  (`KismetSystemLibrary.PrintString` "SendShipInfoCall"))

(fn `AddWeapon`
  (params (WeaponName :type "Name (by ref)"))
  (locals (SoketNameLoopLastIndex :type Integer :default 0))
  (`KismetArrayLibrary.Array_Add` (`self.EquipWeapon`) WeaponName)
  (bind _returnvalue (`|GetDataTableRow` "/Game/Blueprints/Table/DT_WeaponInfo.DT_WeaponInfo" WeaponName)
    (:`then`
      (bind _returnvalue_2 (`KismetArrayLibrary.Array_Length` (`.ShootSoket_28_2F7D8ADC49CDCA8C127E55A6CB2E06E3` (break `/Game/Blueprints/Table/ST_Weapon` _returnvalue))))
      (if (> _returnvalue_2 1)
        (bind _output_get (set `local.SoketNameLoopLastIndex` _returnvalue_2))
        (for _index (range _output_get)
          (bind _returnvalue_3 (`AddComponent|NODE_AddBP_Gun-0` :!label _label))
          (bind _returnvalue_4 (`KismetArrayLibrary.Array_Add` (`self.GunList`) _returnvalue_3))
          (set `/Game/Blueprints/Unit/BP_Gun.GunIndex` _returnvalue_4 _returnvalue_3)
          (bind (_weapontype _damagetype _targettype _shootsoket _projectilemesh _attackdelay _projectilespeed _damagevalue) (break `/Game/Blueprints/Table/ST_Weapon` _returnvalue))
          (set `/Game/Blueprints/Unit/BP_Gun.WeaponType` _weapontype _returnvalue_3)
          (set `/Game/Blueprints/Unit/BP_Gun.DamageType` _damagetype _returnvalue_3)
          (set `/Game/Blueprints/Unit/BP_Gun.TargetType` _targettype _returnvalue_3)
          (set `/Game/Blueprints/Unit/BP_Gun.SoketName` (`|GetArrayItem` _shootsoket _index) _returnvalue_3)
          (set `/Game/Blueprints/Unit/BP_Gun.ProjectileMesh` _projectilemesh _returnvalue_3)
          (set `/Game/Blueprints/Unit/BP_Gun.AttackDelay` _attackdelay _returnvalue_3)
          (set `/Game/Blueprints/Unit/BP_Gun.ProjectileSpeed` _projectilespeed _returnvalue_3)
          (set `/Game/Blueprints/Unit/BP_Gun.DamageValue` _damagevalue _returnvalue_3)
          (`ActorComponent.SetActive` _returnvalue_3 true false)
          (set `/Game/Blueprints/Unit/BP_Gun.GunOwner` self _returnvalue_3))
        (set `local.SoketNameLoopLastIndex` 0)
        (else
          (goto _label))))))

(fn `GetFireTarget`
  (params (TargetActorClass :type "Actor Class Reference") (OriginLoc :type "Vector Structure"))
  (returns (TargetActorRef :type "Actor Object Reference") (IsNotVaild :type Boolean))
  (locals (TargetList :type "Array of Actor Object Reference") (IsNotValid :type Boolean :default true))
  (bind _outactors (`GameplayStatics.GetAllActorsOfClass` TargetActorClass))
  (bind _output_get (set `local.TargetList` _outactors))
  (if (`KismetArrayLibrary.Array_IsNotEmpty` _output_get)
    (bind (_distance _returnvalue) (`GameplayStatics.FindNearestActor` OriginLoc _output_get))
    (`/Engine/EditorBlueprintResources/StandardMacros.IsValid` _returnvalue
      (:`Is Valid`
        (bind _output_get_2 (set `local.IsNotValid` false))
        (return _returnvalue _output_get_2))
      (:`Is Not Valid`
        _)))
  (`KismetSystemLibrary.PrintString` "Find Nearest Actor is Not Valid Actor call")
  (bind _output_get_3 (set `local.IsNotValid` true))
  (return _returnvalue _output_get_3))

(fn `SetShipInfo`
  (params (ShipName :type Name))
  (returns (ItemName :type Name))
  (bind _returnvalue (`|GetDataTableRow` "/Game/Blueprints/Table/DT_ShipInfo.DT_ShipInfo" ShipName)
    (:`then`
      (bind (_mesh _defaultitemname _maxhp) (break `/Game/Blueprints/Table/ST_ShipInfo` _returnvalue))
      (`StaticMeshComponent.SetStaticMesh` (`self.Ship_StaticMesh`) _mesh)
      (bind _output_get (set `self.MaxHp` _maxhp))
      (set `self.CurrentHp` _output_get)
      (return _defaultitemname))))

(fn `SetWeaponInfo`
  (params (RowName :type Name))
  (bind _returnvalue (`|GetDataTableRow` "/Game/Blueprints/Table/DT_WeaponInfo.DT_WeaponInfo" RowName)
    (:`then`
      (bind (_weapontype _damagetype _targettype _shootsoket _projectilemesh _attackdelay _projectilespeed _damagevalue) (break `/Game/Blueprints/Table/ST_Weapon` _returnvalue))
      (switch `/Game/Blueprints/Table/En_WeaponType` _weapontype
        (:`NewEnumerator0`
          (set `self.Projectile Mesh` _projectilemesh)
          (set `self.AttackDelay` _attackdelay)
          (set `self.Projectile Speed` _projectilespeed)
          (set `self.AttackDamage` _damagevalue))))))

(fn `SpawnProjectile`
  (params (ProjectileClass :type "Actor Class Reference") (Scale :type "Vector Structure") (Origin :type "Vector Structure") (TargetLoc :type "Vector Structure"))
  (bind _returnvalue (`|SpawnActorFromClass` ProjectileClass (`KismetMathLibrary.MakeTransform` (.location (`SceneComponent.GetSocketTransform` (`self.Ship_StaticMesh`) "Fire" "RTS_World")) (`KismetMathLibrary.MakeRotator` 0.0 (`/Game/Blueprints/Actor_Mac.Angle_Atan2` Origin TargetLoc)) Scale) "AdjustIfPossibleButAlwaysSpawn" "OverrideRootScale" self self))
  (message `/Game/Blueprints/BP_MainInterface.SetProjectileInfo` _returnvalue (`self.AttackDamage`) 0.0 false)
  (return))

(fn `UserConstructionScript`)