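; Base generator actor that supplies randomized spawn transforms around the player on the XZ plane, apparently for child spawners; it spawns nothing itself.
; On BeginPlay it caches the GameState as BP_EventManager.
; SetRandVec scales Cos and Sin of separate random values by Radius, so offsets are not confined to a circle.
; SetSpawnActerTransform adds that offset to the player's location and pitches it toward the player with slight random jitter.
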(event `self.ReceiveBeginPlay`
  (bind _asbp_event_manager (cast `/Game/Blueprints/BP_EventManager` (`GameplayStatics.GetGameState`)))
  (set `self.RefEventManger` _asbp_event_manager))

(event `self.ReceiveTick`
  (params (DeltaSeconds :type "Float (single-precision)")))

(fn `Set SpawnActerTransform`
  (returns (ReturnValue :type "Transform Structure"))
  (bind (_returnvalue_x _returnvalue_y _returnvalue_z) (`KismetMathLibrary.BreakVector` (`self.K2_GetActorLocation` (`GameplayStatics.GetPlayerPawn` 0))))
  (bind _randvec (`self.SetRandVec`))
  (bind _returnvalue (+ (.x _randvec) _returnvalue_x))
  (bind _returnvalue_2 (+ (.z _randvec) _returnvalue_z))
  (return (`KismetMathLibrary.MakeTransform` (`KismetMathLibrary.MakeVector` _returnvalue 0.0 _returnvalue_2) (`KismetMathLibrary.MakeRotator` 0.0 (`/Game/Blueprints/Actor_Mac.Angle_Atan2` (`KismetMathLibrary.MakeVector` _returnvalue 0.0 _returnvalue_2) (`KismetMathLibrary.MakeVector` _returnvalue_x 0.0 _returnvalue_z) (`KismetMathLibrary.RandomFloatInRange` -10.0 10.0))))))

(fn `SetRandVec`
  (returns (RandVec :type "Vector Structure"))
  (bind _returnvalue (`KismetMathLibrary.RandomFloatInRange` 0.0 360.0))
  (bind _radius (`self.Radius`))
  (bind _output_get (set `self.RandVec` (`KismetMathLibrary.MakeVector` (* (`KismetMathLibrary.Cos` _returnvalue) _radius) 0.0 (* (`KismetMathLibrary.Sin` _returnvalue) _radius))))
  (return _output_get))

(fn `UserConstructionScript`)