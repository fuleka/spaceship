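; Space skybox actor that slowly turns the backdrop around the player, based on the pawn's orientation.
; Each Tick runs MoveRotation, which adds world roll and yaw from the Z and X of the player pawn's up vector, divided by the negated actor X scale.
; The stored location resets to zero after each turn, so the movement check compares against the world origin rather than the previous position.
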(event `self.ReceiveTick`
  (params (DeltaSeconds :type "Float (single-precision)"))
  (`self.MoveRotation`))

(fn `MoveRotation`
  (bind _returnvalue (`GameplayStatics.GetPlayerPawn` 0))
  (bind _returnvalue_x (`KismetMathLibrary.BreakVector` (`self.GetActorScale3D`)))
  (bind (_returnvalue_x_2 _returnvalue_y _returnvalue_z) (`KismetMathLibrary.BreakVector` (`self.GetActorUpVector` _returnvalue)))
  (bind _returnvalue_2 (* _returnvalue_x -1.0))
  (if (not (== (`self.ActorLocTmp`) (`self.K2_GetActorLocation` _returnvalue) :`ErrorTolerance` 0.5))
    (`self.K2_AddActorWorldRotation` (`KismetMathLibrary.MakeRotator` (/ _returnvalue_z _returnvalue_2) 0.0 (/ _returnvalue_x_2 _returnvalue_2)))
    (set `self.ActorLocTmp` (0.0 0.0 0.0))))

(fn `UserConstructionScript`)